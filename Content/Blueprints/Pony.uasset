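; Pony is a target the player runs over in a vehicle to score, tinted a random palette color through a dynamic material on spawn.
; The first overlap from a non-box vehicle component adds a coin through the UI widget, which checks the score.
; That check either stops the Timer or spawns a replacement Pony at a random ground-plane location.
; The hit Pony hides, plays blood and scream effects, then destroys itself.
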(event OnComponentBeginOverlap(Box)
  (params (OverlappedComponent :type Primitive%20Component%20Object%20Reference) (OtherActor :type Actor%20Object%20Reference) (OtherComp :type Primitive%20Component%20Object%20Reference) (OtherBodyIndex :type Integer) (bFromSweep :type Boolean) (SweepResult :type Hit%20Result%20Structure%20%28by%20ref%29))
  (Utilities|Casting|CastToVehicleBlueprint OtherActor)
  (Utilities|Casting|CastToBoxComponent OtherComp
    (:CastFailed
      (Utilities|FlowControl|DoOnce false
        (:Completed
          (bind _foundwidgets (Widget|GetAllWidgetsOfClass "/Game/Blueprints/UI.UI_C" true))
          (Default|ObtainCoin (Utilities|Array|Get(acopy) _foundwidgets))
          (bind _win (Default|CheckScore (Utilities|Array|Get(acopy) _foundwidgets)))
          (if _win
            (bind _returnvalue (Actor|GetActorOfClass "/Game/Blueprints/Timer.Timer_C"))
            (Default|StopTimer _returnvalue)
            (else
              (bind _returnvalue_2 (Game|SpawnActorfromClass "Pony_C" (Math|Transform|MakeTransform "0.000000,0.000000,-1000.000000" "0, 0, 0" "2.000000,2.000000,2.000000") "Undefined" 0 0))
              (CallFunction|SetRandomLocation _returnvalue_2)))
          (Development|SetHiddeninGame (Variables|Default|GetPony) true false)
          (Collision|SetCollisionEnabled (Variables|Default|GetPony) "NoCollision")
          (Components|Activation|Activate (Variables|Default|GetBlood) false)
          (Audio|PlaySound2D "/Game/Audio/SoundFX/PonyScream.PonyScream" 1.0 1.0 0.0 0 0)
          (Utilities|FlowControl|Delay 0.5)
          (Actor|DestroyActor))))))

(event EventBeginPlay
  (bind _returnvalue (Rendering|Material|CreateDynamicMaterialInstance (Variables|Default|GetPony) 4 "/Game/ThirdParty/Pony/Materials/material_0.material_0" "material_0" :!class /Script/Engine.PrimitiveComponent))
  (Rendering|Material|SetVectorParameterValue _returnvalue "Color" (Math|Conversions|ToLinearColor(Color) (Utilities|Array|Get(acopy) (Variables|Default|GetColours) (Math|Random|RandomIntegerinRange 0 9))) :!class /Script/Engine.MaterialInstanceDynamic))

(fn ConstructionScript)

(fn SetRandomLocation
  (params (Pony :type Actor%20Object%20Reference))
  (bind _maxlocationdistance (LocalVariables|GetMaxLocationDistance))
  (bind _returnvalue (* _maxlocationdistance -1.0))
  (Transformation|SetActorLocation Pony (Math|Vector|MakeVector (Math|Random|RandomFloatinRange _returnvalue _maxlocationdistance) (Math|Random|RandomFloatinRange _returnvalue _maxlocationdistance) 0.0) false true))