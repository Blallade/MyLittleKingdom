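; Countdown timer Blueprint that ends the game when time runs out or when stopped.
; StartTimer opens a Tick gate, and DecrementTime counts down minutes, seconds and per-frame "milliseconds", making its speed framerate-dependent, while refreshing the UI widget.
; StopTimer runs once, freezes Player and Car, lowers car volume and shows the end screen.
; After a delay, the widget's score check either triggers the win or reloads MainLevel.
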(event Custom|StartTimer
  (Utilities|FlowControl|Gate true) ; enters at Open
)

(event Custom|StopTimer
  (bind _car (Variables|Default|GetCar))
  (if (not (Variables|Default|GetTimerStopped?))
    (Utilities|FlowControl|Sequence
      (:then_0
        (Variables|Default|SetTimerStopped? true)
        (Utilities|FlowControl|Gate true) ; enters at Close
      )
      (:then_1
        (Variables|/Game/Blueprints/Player.Player_C|SetCanMove (Variables|Default|GetPlayer) false)
        (Variables|/Game/ThirdParty/VehicleAdvBP/Blueprints/VehicleBlueprint.VehicleBlueprint_C|SetCanMove _car false)
        (Default|LowVolume _car)
        (bind _foundwidgets (Widget|GetAllWidgetsOfClass "/Game/Blueprints/UI.UI_C" true))
        (Default|SetTimer (Utilities|Array|Get(acopy) _foundwidgets))
        (Default|ShowEndScreen (Utilities|Array|Get(acopy) _foundwidgets) true)
        (Input|SetInputModeUIOnly (Game|GetPlayerController 0) (Utilities|Array|Get(acopy) _foundwidgets) "DoNotLock")
        (Utilities|FlowControl|Delay 6.0)
        (bind _win (Default|CheckScore (Utilities|Array|Get(acopy) _foundwidgets)))
        (if _win
          (Default|Win (Utilities|Array|Get(acopy) _foundwidgets))
          (Utilities|FlowControl|Delay 2.0)
          (Variables|/Script/Engine.PlayerController|SetbShowMouseCursor (Game|GetPlayerController 0) true)
          (else
            (Game|OpenLevel(byName) "MainLevel")))))))

(event EventTick
  (params (DeltaSeconds :type Float%20%28single-precision%29))
  (Utilities|FlowControl|Gate true
    (:Exit
      (Utilities|DecrementTime
        (:%20%20
          (bind _foundwidgets (Widget|GetAllWidgetsOfClass "/Game/Blueprints/UI.UI_C" true))
          (Default|SetTimer (Utilities|Array|Get(acopy) _foundwidgets)))
        (:End
          (CallFunction|StopTimer))))))

(fn ConstructionScript)