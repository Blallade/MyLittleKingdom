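; Player controller that switches the player between the on-foot character and a car, and handles the press-any-key start prompt.
; Catch possesses the car while in its area, hiding the character and disabling its collision, or exits by restoring it.
; On exit, a line trace along the car's right vector picks that side, or the left if blocked.
; A temporary AnyKey mapping enables character input, hides the start advice, then removes itself.
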(event EventBeginPlay
  (Variables|Default|SetPlayerChar (Game|GetPlayerCharacter 0))
  (Class|InputSettings|AddActionMapping (Class|InputSettings|GetInputSettings) (Utilities|Struct|MakeInputActionKeyMapping "AnyKey" false false false false "AnyKey") true))

(event Input|ActionEvents|InputActionCatch
  (params (Key :type Key%20Structure :default "None"))
  (bind _playerchar (Variables|Default|GetPlayerChar))
  (bind _playerchar_2 (Variables|Default|GetPlayerChar))
  (:Pressed
    (if (Variables|Default|GetInCar)
      (CallFunction|RelocateCharacter)
      (Pawn|Possess (Variables|Default|GetPlayerChar))
      (Rendering|SetActorHiddenInGame _playerchar false)
      (Collision|SetActorEnableCollision _playerchar true)
      (Variables|Default|SetInCar false)
      (elif (Variables|Default|GetInCarArea)
        (Pawn|Possess (Variables|Default|GetCar))
        (Rendering|SetActorHiddenInGame _playerchar_2 true)
        (Collision|SetActorEnableCollision _playerchar_2 false)
        (Variables|Default|SetInCar true)
        (bind _foundwidgets (Widget|GetAllWidgetsOfClass "/Game/Blueprints/UI.UI_C" true))
        (Default|ShowPressEAdvice (Utilities|Array|Get(acopy) _foundwidgets) false)))))

(event Input|ActionEvents|InputActionAnyKey
  (params (Key :type Key%20Structure :default "None"))
  (:Pressed
    (Input|EnableInput (Game|GetPlayerCharacter 0) self)
    (bind _foundwidgets (Widget|GetAllWidgetsOfClass "/Game/Blueprints/UI.UI_C" true))
    (Default|HideStartAdvice (Utilities|Array|Get(acopy) _foundwidgets))
    (Class|InputSettings|RemoveActionMapping (Class|InputSettings|GetInputSettings) (Utilities|Struct|MakeInputActionKeyMapping "AnyKey" false false false false "AnyKey") true)))

(fn ConstructionScript)

(fn RelocateCharacter
  (bind _car (Variables|Default|GetCar))
  (bind _returnvalue (Transformation|GetActorLocation _car))
  (bind _positionable (CallFunction|CheckifCanLocate))
  (Transformation|SetActorLocationAndRotation (Variables|Default|GetPlayerChar) (+ (Math|Vector|MakeVector (.x _returnvalue) (.y _returnvalue) (.z (Transformation|GetActorLocation (Variables|Default|GetPlayerChar)))) (* (Transformation|GetActorRightVector _car) (select _positionable 2e+02 -2e+02))) (Pawn|GetControlRotation :!class /Script/Engine.Controller) false true))

(fn CheckifCanLocate
  (bind _car (Variables|Default|GetCar))
  (bind _returnvalue (Transformation|GetActorLocation _car))
  (bind _returnvalue_2 (Collision|LineTraceForObjects _returnvalue (+ _returnvalue (* (Transformation|GetActorRightVector _car) 4e+02)) (Utilities|Array|MakeArray "ObjectTypeQuery1" "ObjectTypeQuery2" "ObjectTypeQuery5") false 0 "None"))
  (return (not _returnvalue_2)))